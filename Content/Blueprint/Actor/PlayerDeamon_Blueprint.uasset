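; Player demon actor Blueprint that adds blood effects when its attack hitbox hits actors tagged "Enemy".
; The overlap spawns a blood splatter emitter at the enemy's location and binds to its particle collision event.
; Each collision spawns a short-lived, randomly sized decal aligned to the surface normal, using a dynamic material instance with a random "Frame" parameter for variation.
; The charge collision overlap and Tick events are empty.
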(event `self.attackHitBox.OnComponentBeginOverlap`
  (params (OverlappedComponent :type "PrimitiveComponent Object Reference") (OtherActor :type "Actor Object Reference") (OtherComp :type "PrimitiveComponent Object Reference") (OtherBodyIndex :type Integer) (bFromSweep :type Boolean) (SweepResult :type "HitResult Structure (by ref)"))
  (if (`KismetSystemLibrary.IsValid` OtherActor)
    (if (`self.ActorHasTag` OtherActor "Enemy")
      (bind _returnvalue (`GameplayStatics.SpawnEmitterAtLocation` "/Game/Effects/BloodSplatter.BloodSplatter" (`self.K2_GetActorLocation` OtherActor)))
      (add `ParticleSystemComponent.OnParticleCollide` _returnvalue (delegate `On Collide Event`)))))

(event `On Collide Event`
  (params (EventName :type Name) (EmitterTime :type "Float (double-precision)") (ParticleTime :type Integer) (Location :type "Vector Structure") (Velocity :type "Vector Structure") (Direction :type "Vector Structure") (Normal :type "Vector Structure") (BoneName :type Name) (PhysMat :type "PhysicalMaterial Object Reference"))
  (bind _returnvalue (`KismetMaterialLibrary.CreateDynamicMaterialInstance` "/Game/Effects/MatAndTexture/BloodSplatterMat.BloodSplatterMat"))
  (`MaterialInstanceDynamic.SetScalarParameterValue` _returnvalue "Frame" (`KismetMathLibrary.Conv_IntToDouble` (`KismetMathLibrary.RandomInteger` 11)))
  (`GameplayStatics.SpawnDecalAtLocation` _returnvalue (`KismetMathLibrary.Conv_DoubleToVector` (`KismetMathLibrary.RandomFloatInRange` 10.0 20.0)) Location (`KismetMathLibrary.MakeRotFromX` Normal) 5.0))

(event `self.collisionCharge.OnComponentBeginOverlap`
  (params (OverlappedComponent :type "PrimitiveComponent Object Reference") (OtherActor :type "Actor Object Reference") (OtherComp :type "PrimitiveComponent Object Reference") (OtherBodyIndex :type Integer) (bFromSweep :type Boolean) (SweepResult :type "HitResult Structure (by ref)")))

(event `self.ReceiveTick`
  (params (DeltaSeconds :type "Float (single-precision)")))

(fn `UserConstructionScript`)