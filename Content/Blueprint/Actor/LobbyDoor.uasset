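; LobbyDoor is an actor that a human player can remove by releasing Jump while standing in its collision area.
; Overlap by the player's capsule sets a flag, enables input from player controller 0 and shows a text render by scaling its X to one.
; Leaving clears the flag, plays a click sound and collapses the text, but input stays enabled.
; The Jump handler checks the flag, clears it and destroys the actor.
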(event `self.Collision.OnComponentBeginOverlap`
  (params (OverlappedComponent :type "PrimitiveComponent Object Reference") (OtherActor :type "Actor Object Reference") (OtherComp :type "PrimitiveComponent Object Reference") (OtherBodyIndex :type Integer) (bFromSweep :type Boolean) (SweepResult :type "HitResult Structure (by ref)"))
  (cast `/Game/Blueprint/Actor/PlayerHuman_Blueprint` OtherActor)
  (cast `CapsuleComponent` OtherComp)
  (`|ExecutionSequence`
    (:`then_0`
      (set `self.IsOverlapping` true))
    (:`then_1`
      (`self.EnableInput` (`GameplayStatics.GetPlayerController` 0)))
    (:`then_2`
      (`TextRenderComponent.SetXScale` (`self.TextRender`) 1.0))))

(event `self.Collision.OnComponentEndOverlap`
  (params (OverlappedComponent :type "PrimitiveComponent Object Reference") (OtherActor :type "Actor Object Reference") (OtherComp :type "PrimitiveComponent Object Reference") (OtherBodyIndex :type Integer))
  (cast `/Game/Blueprint/Actor/PlayerHuman_Blueprint` OtherActor)
  (cast `CapsuleComponent` OtherComp)
  (if (`self.IsOverlapping`)
    (`|ExecutionSequence`
      (:`then_0`
        (set `self.IsOverlapping` false))
      (:`then_1`
        (`GameplayStatics.PlaySound2D` "/Game/Sounds/ButtonClick.ButtonClick" 1.0 1.0 0.0 null null))
      (:`then_2`
        (`TextRenderComponent.SetXScale` (`self.TextRender`) 0.0)))))

(event `InputAction|Jump`
  (params (Key :type "Key Structure"))
  (:`Released`
    (if (`self.IsOverlapping`)
      (`|ExecutionSequence`
        (:`then_0`
          (set `self.IsOverlapping` false))
        (:`then_1`
          (`self.K2_DestroyActor`))))))

(fn `UserConstructionScript`)