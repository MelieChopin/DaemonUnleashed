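; Game mode Blueprint that handles pausing and resuming the game from the Start input action.
; BeginPlay enables input from the first player controller on the game mode itself.
; Pressing Start while the game state is RUN or PAUSE calls SetUnsetPause, which toggles the engine pause and sets MyGameState to match.
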(event `self.ReceiveBeginPlay`
  (`self.EnableInput` (`GameplayStatics.GetPlayerController` 0)))

(event `self.ReceiveTick`
  (params (DeltaSeconds :type "Float (single-precision)")))

(event `InputAction|Start` :paused true
  (params (Key :type "Key Structure"))
  (bind _mygamestate (`self.myGameState`))
  (:`Pressed`
    (if (or (`|EnumEquality` _mygamestate "RUN") (`|EnumEquality` _mygamestate "PAUSE"))
      (`self.SetUnsetPause`))))

(fn `SetUnsetPause`
  (if (`GameplayStatics.IsGamePaused`)
    (`GameplayStatics.SetGamePaused` false)
    (set `self.myGameState` "RUN")
    (else
      (`GameplayStatics.SetGamePaused` true)
      (set `self.myGameState` "PAUSE"))))

(fn `UserConstructionScript`)